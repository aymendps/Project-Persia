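; Side-view camera actor that follows the player character, zooms and handles screen fades.
; While following is enabled, Tick interpolates it toward the player plus a forward-vector look-ahead, with the offset's Y zeroed to avoid unintended zoom.
; Zoom events use a timeline to blend the spring arm's Y socket offset between default and in/out values.
; One level sequence fades in on BeginPlay when played in reverse, and out when played forward.
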(event `self.ReceiveBeginPlay`
  ;[1 1 1] Fade in camera on begin play
  (bind _outactor (`LevelSequencePlayer.CreateLevelSequencePlayer` "/Game/MyContent/Sequences/LS_FadeSequence.LS_FadeSequence"))
  (set `self.FadeSequencePlayer` (`LevelSequenceActor.SequencePlayer` _outactor))
  (`self.FadeInCamera`))

(event `self.ReceiveTick`
  (params (DeltaSeconds :type "Float (single-precision)"))
  ;[1 1 1] Camera Movement
  (`self.UpdateCameraLocation`))

(event `ZoomCamera`
  (params (`ZoomIn?` :type Boolean))
  ;[1 1 1] Zoom camera in/out by decreasing/increasing the spring's arm socket offset over time
  (bind (_direction _lerp_alpha) (`Timeline|Lerp Timeline` :!via `PlayFromStart`)
    (:`Update`
      (set `SpringArmComponent.SocketOffset` (`KismetMathLibrary.MakeVector` 0.0 (`KismetMathLibrary.Lerp` (`self.DefaultOffset`) (`KismetMathLibrary.SelectFloat` (`self.ZoomInOffset`) (`self.ZoomOutOffset`) `ZoomIn?`) _lerp_alpha)) (`self.SpringArm`)))))

(event `RevertZoomCamera`
  (params (`FromZoomIn?` :type Boolean))
  ;[1 1 1] Revert to the spring's arm default socket offset back from zoom in/out over time
  (`TimelineComponent.ReverseFromEnd` (`self.Lerp Timeline`))
  (set `SpringArmComponent.SocketOffset` (`KismetMathLibrary.MakeVector` 0.0 (`KismetMathLibrary.Lerp` (`KismetMathLibrary.SelectFloat` (`self.ZoomInOffset`) (`self.ZoomOutOffset`) `FromZoomIn?`) (`self.DefaultOffset`))) (`self.SpringArm`)))

(fn `FadeInCamera`
  (`MovieSceneSequencePlayer.PlayReverse` (`self.FadeSequencePlayer`)))

(fn `FadeOutCamera`
  (`MovieSceneSequencePlayer.Play` (`self.FadeSequencePlayer`)))

(fn `InitializeCameraLocation`
  (bind _playercharacter (`self.PlayerCharacter`))
  (bind (_returnvalue_x _returnvalue_y _returnvalue_z) (`KismetMathLibrary.BreakVector` (* (`self.GetActorForwardVector` _playercharacter) (`self.TargetOffset`))))
  (`self.K2_SetActorLocation` (+ (`self.K2_GetActorLocation` _playercharacter) (`KismetMathLibrary.MakeVector` _returnvalue_x 0.0 _returnvalue_z))))

(fn `UpdateCameraLocation`
  (bind _playercharacter (`self.PlayerCharacter`))
  (bind (_returnvalue_x _returnvalue_y _returnvalue_z) (`KismetMathLibrary.BreakVector` (* (`self.GetActorForwardVector` _playercharacter) (`self.TargetOffset`))))
  ;[1 1 1] Move towards target location over time as long as Should Follow Target is true
  (if (`self.ShouldFollowTarget`)
    (`self.K2_SetActorLocation` (`KismetMathLibrary.VInterpTo` (`self.K2_GetActorLocation`) (+ (`self.K2_GetActorLocation` _playercharacter) (`KismetMathLibrary.MakeVector` _returnvalue_x 0.0 _returnvalue_z)) (`GameplayStatics.GetWorldDeltaSeconds`) (`self.CameraSpeed`)))))

(fn `UserConstructionScript`
  (set `SpringArmComponent.SocketOffset` (`KismetMathLibrary.MakeVector` 0.0 (`self.DefaultOffset`)) (`self.SpringArm`)))