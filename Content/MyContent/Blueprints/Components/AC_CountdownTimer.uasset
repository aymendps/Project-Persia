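; AC_CountdownTimer is a component that runs a minutes-and-seconds countdown and triggers game loss when it expires.
; Each Tick event, unless paused, takes one second off, borrowing from minutes when seconds are zero.
; A tick at 00:00 pauses the timer and calls EventGameLost on the first player's BP_PlayerController.
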(event `self.ReceiveTick`
  (params (DeltaSeconds :type "Float (single-precision)"))
  (if (not (`self.IsPaused`))
    ;[1 1 1] If we can decrement seconds
    (if (!= (`self.Seconds`) 0)
      (`/Engine/EditorBlueprintResources/StandardMacros.DecrementInt` (`self.Seconds`))
      (else
        ;[1 1 1] If we can decrement minutes
        (if (!= (`self.Minutes`) 0)
          (`/Engine/EditorBlueprintResources/StandardMacros.DecrementInt` (`self.Minutes`)
            (:`  `
              (set `self.Seconds` 59)))
          (else
            ;[1 1 1] We can't decrement neither seconds nor minutes, so timer is 00:00
            (`self.CountdownTimerHasRunOut`)))))))

(event `CountdownTimerHasRunOut`
  ;[1 1 1] Call when countdown timer becomes 00:00
  (set `self.IsPaused` true)
  (bind _asbp_player_controller (cast `/Game/MyContent/Blueprints/GameMode/BP_PlayerController` (`GameplayStatics.GetPlayerController` 0)))
  (`/Game/MyContent/Blueprints/GameMode/BP_PlayerController.Event GameLost` _asbp_player_controller))