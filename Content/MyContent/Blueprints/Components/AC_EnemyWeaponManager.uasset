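; Actor component that manages an enemy character's sword, spawning it on the owner and handling equip and unequip.
; On BeginPlay it caches the owning AI_EnemyCharacter and attaches a new BP_EnemyWeapon to the mesh's unequip socket.
; EquipSword and UnequipSword play montages whose notifies move the scimitar mesh between sockets in time with the animation.
; Each notify also sets IsWeaponEquipped and passes it to the AI controller's key update.
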(event `self.ReceiveBeginPlay`
  ;[1 1 1] Cache reference to enemy character that owns this
  (bind _asai_enemy_character (cast `/Game/MyContent/Blueprints/Characters/Enemy/AI_EnemyCharacter` (`self.GetOwner`)))
  (bind _output_get (set `self.EnemyCharacter` _asai_enemy_character))
  ;[1 1 1] Attach weapon to enemy character, ready to be equipped
  (bind _returnvalue (`|SpawnActorFromClass` "/Game/MyContent/Blueprints/Props/Weapons/BP_EnemyWeapon.BP_EnemyWeapon_C" (`SceneComponent.GetSocketTransform` (`Character.Mesh` _output_get) "weapon_unequip_socket" "RTS_World") "AlwaysSpawn" "MultiplyWithRoot" null (`self.EnemyCharacter`) null))
  (bind _output_get_2 (set `self.EnemyWeapon` _returnvalue))
  (`Actor.K2_AttachToComponent` _output_get_2 (`Character.Mesh` (`self.EnemyCharacter`)) "weapon_unequip_socket" "SnapToTarget" "SnapToTarget" "SnapToTarget" true))

(event `EquipSword`
  (`|PlayMontage` (`Character.Mesh` (`self.EnemyCharacter`)) "/Game/MyContent/Animations/FightRelated/Idle/AM_Idle_Equip.AM_Idle_Equip"
    (:`OnNotifyBegin`
      ;[1 1 1] Equip sword the moment the hand takes it
      (`SceneComponent.K2_AttachToComponent` (`/Game/MyContent/Blueprints/Props/Weapons/BP_ScimitarWeapon.SM_Scimitar` (`self.EnemyWeapon`)) (`Character.Mesh` (`self.EnemyCharacter`)) "weapon_equip_socket" "SnapToTarget" "SnapToTarget" "SnapToTarget" true)
      (bind _output_get (set `self.IsWeaponEquipped` true))
      (`/Game/MyContent/Blueprints/Characters/Enemy/AIC_EnemyCharacter.UpdateIsWeaponEquippedKey` (`/Game/MyContent/Blueprints/Characters/Enemy/AI_EnemyCharacter.AIController` (`self.EnemyCharacter`)) _output_get))))

(event `UnequipSword`
  (`|PlayMontage` (`Character.Mesh` (`self.EnemyCharacter`)) "/Game/MyContent/Animations/FightRelated/Idle/AM_Idle_Unequip.AM_Idle_Unequip"
    (:`OnNotifyBegin`
      ;[1 1 1] Unequip the sword the moment the sword is laying on the side
      (`SceneComponent.K2_AttachToComponent` (`/Game/MyContent/Blueprints/Props/Weapons/BP_ScimitarWeapon.SM_Scimitar` (`self.EnemyWeapon`)) (`Character.Mesh` (`self.EnemyCharacter`)) "weapon_unequip_socket" "SnapToTarget" "SnapToTarget" "SnapToTarget" true)
      (bind _output_get (set `self.IsWeaponEquipped` false))
      (`/Game/MyContent/Blueprints/Characters/Enemy/AIC_EnemyCharacter.UpdateIsWeaponEquippedKey` (`/Game/MyContent/Blueprints/Characters/Enemy/AI_EnemyCharacter.AIController` (`self.EnemyCharacter`)) _output_get))))