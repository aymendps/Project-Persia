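; Player character component that plays a death montage matching the damage type and returns a delay, apparently used before reloading.
; It caches its BP_PlayerCharacter owner, then dispatches on the DamageTypeBase identifier to Falling or Spikes handlers.
; Spike deaths switch to the flat-fall impact montage and its shorter delay when FallingDamage reports a high falling speed.
; A failed damage type cast plays the default montage and returns the default delay.
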(event `self.ReceiveBeginPlay`
  ;[1 1 1] Cache reference to the player character that owns this component
  (bind _asbp_player_character (cast `/Game/MyContent/Blueprints/Characters/Player/BP_PlayerCharacter` (`self.GetOwner`))
    (:`then`
      (set `self.PlayerCharacter` _asbp_player_character))
    (:`CastFailed`
      (`KismetSystemLibrary.PrintString` "Owner of PlayerDeath is not of type BP_PlayerCharacter" true true (struct :`R` 1.0 :`A` 1.0)))))

(fn `PlayDeathAnimMontage`
  (params (DamageType :type "DamageType Object Reference"))
  (returns (DelayBeforeReloading :type "Float (double-precision)"))
  (bind _asdamage_type_base (cast `DamageTypeBase` DamageType)
    (:`then`
      (switch `EDamageTypeIdentifier` (`DamageTypeBase.DamageTypeIdentifier` _asdamage_type_base)
        (:`Falling`
          (bind _delaybeforereloading (`self.PlayFallingDeathAnim`))
          (return _delaybeforereloading))
        (:`Spikes`
          (bind _delaybeforereloading_2 (`self.PlaySpikesDeathAnim`))
          (return _delaybeforereloading_2))))
    (:`CastFailed`
      ;[1 1 1] In case the damage type is unknown, play the default montage and return the default delay
      (`KismetSystemLibrary.PrintString` "Damage Type Is Unknown" true true (struct :`R` 1.0 :`A` 1.0))
      (`Character.PlayAnimMontage` (`self.PlayerCharacter`) (`self.DefaultDeathAnim`) 1.0 "None")
      (return (`self.DefaultDelayBeforeReloading`)))))

(fn `PlayFallingDeathAnim`
  (returns (DelayBeforeReloading :type "Float (double-precision)"))
  (locals (NormalFallingSpeed :type "Float (double-precision)" :default 1800.0))
  (`Character.PlayAnimMontage` (`self.PlayerCharacter`) "/Game/MyContent/Blueprints/Characters/Player/Animations/AM_FlatFalling_Impact.AM_FlatFalling_Impact" 1.0 "None")
  (return 0.2))

(fn `PlaySpikesDeathAnim`
  (returns (DelayBeforeReloading :type "Float (double-precision)"))
  (locals (NormalFallingSpeed :type "Float (double-precision)" :default 1800.0))
  (bind _returnvalue (>= (`FallingDamageComponent.CurrentFallingSpeed` (`/Game/MyContent/Blueprints/Characters/Player/BP_PlayerCharacter.FallingDamage` (`self.PlayerCharacter`))) (`local.NormalFallingSpeed`)))
  (`Character.PlayAnimMontage` (`self.PlayerCharacter`) (select `bool` _returnvalue :`false` "/Game/MyContent/Blueprints/Characters/Player/Animations/AM_DyingToSpikes.AM_DyingToSpikes" :`true` "/Game/MyContent/Blueprints/Characters/Player/Animations/AM_FlatFalling_Impact.AM_FlatFalling_Impact" :!type "AnimMontage Object Reference") 1.0 "None")
  (return (select `bool` _returnvalue :`false` 0.8 :`true` 0.2)))