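; Player weapon manager component that spawns the sword and handles equipping and unequipping it between two mesh sockets.
; Equip and unequip play montages whose notifies reattach the sword, with input disabled until the montage completes.
; Each transition resets the attack index and switches walk speed and orient-to-movement.
; When equipping, it smoothly rotates the player to the nearer of forward or backward along the direction vector and stores that sign.
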(event `self.ReceiveBeginPlay`
  ;[1 1 1] Cache reference to the player character and its player controller and spawn the player's sword if they already have found and taken it.
  (set `self.PlayerCharacter` (cast `/Game/MyContent/Blueprints/Characters/Player/BP_PlayerCharacter` (`GameplayStatics.GetPlayerCharacter` 0) :!pure true))
  (set `self.PlayerController` (cast `/Game/MyContent/Blueprints/GameMode/BP_PlayerController` (`GameplayStatics.GetPlayerController` 0) :!pure true))
  (if (`self.HasSword`)
    (`self.SpawnSword` false)))

(event `SpawnSword`
  (params (`SpawnEquipped?` :type Boolean :default true))
  ;[1 1 1] Spawn sword using the socket's transform and then attach it to the same socket
  (`/Engine/EditorBlueprintResources/StandardMacros.IsValid` (`self.PlayerSword`)
    (:`Is Not Valid`
      (`self.AttachSwordToPlayer` `SpawnEquipped?`)
      (set `self.HasSword` true)
      (set `self.IsWeaponEquipped` `SpawnEquipped?`))))

(event `EnterTransition`
  (params (`IsUnequipping?` :type Boolean))
  (bind (_fightdirectionsign _nearestrotationtovector) (`self.FindNearestPlayerDirection`))
  (bind _playercharacter (`self.PlayerCharacter`))
  (bind _playercharacter_2 (`self.PlayerCharacter`))
  ;[1 1 1] Don't let the player take another action while equipping/unequipping
  (set `/Game/MyContent/Blueprints/GameMode/BP_PlayerController.bEnableInput` false (`self.PlayerController`))
  (set `self.IsInTransition` true)
  ;[1 1 1] Since player used this instead of attack, reset the attack index to 0
  (set `/Game/MyContent/Blueprints/Characters/Player/BP_PlayerCharacter.AttackIndex` 0 (`self.PlayerCharacter`))
  ;[1 1 1] If player is unequipping, set max walk speed back to the default value, otherwise set it to the fighting value
  (set `CharacterMovementComponent.MaxWalkSpeed` (`KismetMathLibrary.SelectFloat` (`/Game/MyContent/Blueprints/Characters/Player/BP_PlayerCharacter.MaxWalkSpeed` _playercharacter) (`/Game/MyContent/Blueprints/Characters/Player/BP_PlayerCharacter.MaxFightWalkSpeed` _playercharacter) `IsUnequipping?`) (`Character.CharacterMovement` _playercharacter))
  ;[1 1 1] If equipping, we should stop orienting rotation to movement, since player has to face same direction when going forward/backward
  (bind _output_get (set `CharacterMovementComponent.bOrientRotationToMovement` `IsUnequipping?` (`Character.CharacterMovement` (`self.PlayerCharacter`))))
  ;[1 1 1] If equipping, we should rotate the player to look completely forward or backward depending on what's nearest. Since rotation will no longer change depending on movement, we can't risk the player to be stuck facing left or right
  (if (not _output_get)
    ;;[1 1 1] Equal to 1 if player is looking forward, and -1 if looking backward
    (set `/Game/MyContent/Blueprints/Characters/Player/BP_PlayerCharacter.FightDirectionSign` _fightdirectionsign (`self.PlayerCharacter`))
    (`KismetSystemLibrary.MoveComponentTo` (`Character.CapsuleComponent` _playercharacter_2) (`Actor.K2_GetActorLocation` _playercharacter_2) _nearestrotationtovector true true 0.2 true)))

(event `ExitTransition`
  ;[1 1 1] Allow player to take other actions now that equipping/unequipping is done
  (set `/Game/MyContent/Blueprints/GameMode/BP_PlayerController.bEnableInput` true (`self.PlayerController`))
  (set `self.IsInTransition` false)
  (set `/Game/MyContent/Blueprints/Characters/Player/BP_PlayerCharacter.IsExecFightAction` false (`self.PlayerCharacter`)))

(event `EquipSword`
  (if (and (not (`self.IsWeaponEquipped`)) (`self.HasSword`) (not (`self.IsInTransition`)))
    (`self.EnterTransition` false)
    (`|PlayMontage` (`Character.Mesh` (`self.PlayerCharacter`)) "/Game/MyContent/Animations/FightRelated/Idle/AM_Idle_Equip.AM_Idle_Equip"
      (:`OnCompleted`
        (`self.ExitTransition`))
      (:`OnNotifyBegin`
        ;[1 1 1] Equip sword the moment player's hand takes it
        (`SceneComponent.K2_AttachToComponent` (`/Game/MyContent/Blueprints/Props/Weapons/BP_ScimitarWeapon.SM_Scimitar` (`self.PlayerSword`)) (`Character.Mesh` (`self.PlayerCharacter`)) "weapon_equip_socket" "SnapToTarget" "SnapToTarget" "SnapToTarget" true)
        (set `self.IsWeaponEquipped` true)))))

(event `UnequipSword`
  (if (and (`self.IsWeaponEquipped`) (`self.HasSword`) (not (`self.IsInTransition`)))
    (`self.EnterTransition` true)
    (`|PlayMontage` (`Character.Mesh` (`self.PlayerCharacter`)) "/Game/MyContent/Animations/FightRelated/Idle/AM_Idle_Unequip.AM_Idle_Unequip"
      (:`OnCompleted`
        (`self.ExitTransition`))
      (:`OnNotifyBegin`
        ;[1 1 1] Unequip the sword the moment the sword is laying on the side of the player
        (`SceneComponent.K2_AttachToComponent` (`/Game/MyContent/Blueprints/Props/Weapons/BP_ScimitarWeapon.SM_Scimitar` (`self.PlayerSword`)) (`Character.Mesh` (`self.PlayerCharacter`)) "weapon_unequip_socket" "SnapToTarget" "SnapToTarget" "SnapToTarget" true)
        (set `self.IsWeaponEquipped` false)))))

(fn `AttachSwordToPlayer`
  (params (AttachAsEquipped :type Boolean))
  (bind _returnvalue (`|SpawnActorFromClass` "/Game/MyContent/Blueprints/Props/Weapons/BP_PlayerWeapon.BP_PlayerWeapon_C" (`SceneComponent.GetSocketTransform` (`Character.Mesh` (`self.PlayerCharacter`)) (select `bool` AttachAsEquipped :`false` "weapon_unequip_socket" :`true` "weapon_equip_socket" :!type "Name") "RTS_World") "AlwaysSpawn" "MultiplyWithRoot" null (`self.PlayerCharacter`) null))
  (bind _output_get (set `self.PlayerSword` _returnvalue))
  (`Actor.K2_AttachToComponent` _output_get (`Character.Mesh` (`self.PlayerCharacter`)) (select `bool` AttachAsEquipped :`false` "weapon_unequip_socket" :`true` "weapon_equip_socket" :!type "Name") "SnapToTarget" "SnapToTarget" "SnapToTarget" true))

(fn `FindNearestPlayerDirection`
  (returns (FightDirectionSign :type "Float (double-precision)") (NearestRotationToVector :type "Rotator Structure"))
  (bind _playercharacter (`self.PlayerCharacter`))
  (bind _returnvalue (< (`MathUtility.AngleBetweenVectors` (`Actor.GetActorForwardVector` _playercharacter) (`/Game/MyContent/Blueprints/Characters/Player/BP_PlayerCharacter.DirectionVector` _playercharacter)) (`MathUtility.AngleBetweenVectors` (`Actor.GetActorForwardVector` _playercharacter) (* (`/Game/MyContent/Blueprints/Characters/Player/BP_PlayerCharacter.DirectionVector` _playercharacter) -1.0))))
  ;[1 1 1] If the player is looking more towards the default direction vector, then return the rotation when the player is completely facing the default direction vector.
  ; Otherwise, provide the rotation that makes the player face the opposite of default direction vector.
  ; Also return the direction sign: 1 if the player will be rotated towards the default direction vector, or -1 if player will be rotated to the opposite vector.
  (return (`KismetMathLibrary.SelectFloat` 1.0 -1.0 _returnvalue) (`KismetMathLibrary.SelectRotator` (struct :`Yaw` 180.0) (struct) _returnvalue)))