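; Cell door that slides vertically open or closed, once, when something first overlaps its trigger.
; The construction script derives travel distance from mesh bounds plus an offset, sets start and target locations from StartsOpen, and shows the matching direction arrow.
; The overlap fires DoorTriggerActivated, which plays a timeline at DoorSpeed rate to lerp the mesh's relative location to the target.
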(event `self.DoorTrigger.OnComponentBeginOverlap`
  (params (OverlappedComponent :type "PrimitiveComponent Object Reference") (OtherActor :type "Actor Object Reference") (OtherComp :type "PrimitiveComponent Object Reference") (OtherBodyIndex :type Integer) (bFromSweep :type Boolean) (SweepResult :type "HitResult Structure (by ref)"))
  ;[1 1 1] Invoke the DoorTriggerActivated event
  ;;[1 1 1] Only proceed if the player is yet to activate the door trigger
  (if (not (`self.bIsActivated`))
    (set `self.bIsActivated` true)
    (`self.Door Trigger Activated`)))

(event `Door Trigger Activated`
  ;[1 1 1] Move the door smoothly from its initial location to the target location, so it opens/closes
  (bind (_direction _lerp_alpha) (`Timeline|Lerp Timeline`)
    (:`Update`
      (`self.MoveDoorSmoothly` _lerp_alpha))))

(fn `CalculateDoorHeight`
  (bind (_min _max) (`StaticMeshComponent.GetLocalBounds` (`self.SM_Cell_Door`)))
  ;[1 1 1] Subtract the bottom bound from the top bound to get the door height. Then add the height offset before setting its value
  (set `self.DoorHeight` (+ (`self.DoorHeightOffset`) (- (.z _max) (.z _min)))))

(fn `CalculateDoorInitialLocation`
  (bind (_relativelocation_x _relativelocation_y _relativelocation_z) (`KismetMathLibrary.BreakVector` (`SceneComponent.RelativeLocation` (`self.SM_Cell_Door`))))
  ;[1 1 1] If the door starts open, then update its relative location so it becomes open.
  (if (`self.bStartsOpen`)
    ;[1 1 1] Move the door's relative location upwards instantly using the door height, so that it starts open
    (bind _output_get (set `self.DoorInitialLocation` (`KismetMathLibrary.MakeVector` _relativelocation_x _relativelocation_y (+ _relativelocation_z (`self.DoorHeight`)))))
    (`SceneComponent.K2_SetRelativeLocation` (`self.SM_Cell_Door`) _output_get false false)
    (else
      ;[1 1 1] Just set the value of initial location to the current relative location since the door starts closed, which is the default state
      (set `self.DoorInitialLocation` (`SceneComponent.RelativeLocation` (`self.SM_Cell_Door`))))))

(fn `CalculateDoorTargetLocation`
  (bind (_relativelocation_x _relativelocation_y _relativelocation_z) (`KismetMathLibrary.BreakVector` (`SceneComponent.RelativeLocation` (`self.SM_Cell_Door`))))
  ;[1 1 1] If the door is initially open, multiply the door's height by -1 so that adding it with the door's relative location will result in subtracting it instead, otherwise keep the value of the door height as is. This will result in finding the correct target location depending on if the door is going to open or close.
  (set `self.DoorTargetLocation` (`KismetMathLibrary.MakeVector` _relativelocation_x _relativelocation_y (+ _relativelocation_z (`KismetMathLibrary.SelectFloat` (* (`self.DoorHeight`) -1.0) (`self.DoorHeight`) (`self.bStartsOpen`))))))

(fn `MoveDoorSmoothly`
  (params (Alpha :type "Float (single-precision)"))
  ;[1 1 1] Use the timeline alpha to lerp from the initial location to the target location, then using the result to move the relative location of the door
  (`SceneComponent.K2_SetRelativeLocation` (`self.SM_Cell_Door`) (`KismetMathLibrary.VLerp` (`self.DoorInitialLocation`) (`self.DoorTargetLocation`) Alpha) false false))

(fn `Show Door Direction Arrow`
  ;[1 1 1] Show the Opening Arrow if the door starts closed. Show the Closing Arrow if the door starts open
  (`SceneComponent.SetVisibility` (`self.Closing Arrow`) (`self.bStartsOpen`) false)
  (`SceneComponent.SetVisibility` (`self.Opening Arrow`) (not (`self.bStartsOpen`)) false))

(fn `UserConstructionScript`
  ;[1 1 1] Initialize door depending on chosen settings
  (`self.Show Door Direction Arrow`)
  (`self.CalculateDoorHeight`)
  (`self.CalculateDoorInitialLocation`)
  (`self.CalculateDoorTargetLocation`)
  (`TimelineComponent.SetPlayRate` (`self.Lerp Timeline`) (`self.DoorSpeed`)))