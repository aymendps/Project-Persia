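; BP_DefaultGameMode is the game mode that handles level transitions and level restarts with a camera fade.
; It caches the BP_PlayerCharacter on BeginPlay.
; LoadLevel stops the character's camera manager from following, fades to black, waits briefly, then opens the named level.
; ReloadThisLevel, intended for player death, passes the current level name to LoadLevel.
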(event `self.ReceiveBeginPlay`
  ;[1 1 1] Cache reference to the player character
  (set `self.Player Character` (cast `/Game/MyContent/Blueprints/Characters/Player/BP_PlayerCharacter` (`GameplayStatics.GetPlayerCharacter` 0) :!pure true)))

(event `Event LoadLevel`
  (params (LevelToLoad :type Name))
  (bind _playercameramanager (`/Game/MyContent/Blueprints/Characters/Player/BP_PlayerCharacter.PlayerCameraManager` (`self.Player Character`)))
  ;[1 1 1] LoadLevel - Call when loading a level instead of OpenLevel to play sequence first
  ;;[1 1 1] Stop and fade out camera view to black
  (set `/Game/MyContent/Blueprints/Cameras/BP_PlayerCameraManager.ShouldFollowTarget` false _playercameramanager)
  (`/Game/MyContent/Blueprints/Cameras/BP_PlayerCameraManager.FadeOutCamera` _playercameramanager)
  (`KismetSystemLibrary.Delay` 2.0)
  (`GameplayStatics.OpenLevel` LevelToLoad))

(event `Event ReloadThisLevel`
  ;[1 1 1] ReloadThisLevel - Call when a player dies to restart this level
  (bind _returnvalue (`GameplayStatics.GetCurrentLevelName` true))
  (`self.Event LoadLevel` (`KismetStringLibrary.Conv_StringToName` _returnvalue)))

(fn `UserConstructionScript`)