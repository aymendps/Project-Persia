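; Main menu controller that shows the title UI and starts the transition toward the tutorial level when any key is pressed.
; BeginPlay adds the UMG_MainMenu widget to the viewport and sets the camera timeline's play rate.
; The first key press, gated by DoOnce, triggers the widget's transition, destroys the title smoke and plays a timeline that lerps the menu camera's height from initial to final.
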(event `self.ReceiveBeginPlay`
  ;[1 1 1] Display main menu UI
  (bind _returnvalue (`|CreateWidget` "/Game/MyContent/Blueprints/Widgets/UMG_MainMenu.UMG_MainMenu_C"))
  (bind _output_get (set `self.MainMenuHUD` _returnvalue))
  (`UserWidget.AddToViewport` _output_get 0)
  (`TimelineComponent.SetPlayRate` (`self.CameraTransitionTimeline`) (`self.CameraTransitionPlayRate`)))

(event `Key|AnyKey`
  (params (Key :type "Key Structure"))
  (bind _mainmenucamera (`self.MainMenuCamera`))
  (bind (_returnvalue_x _returnvalue_y) (`KismetMathLibrary.BreakVector` (`self.K2_GetActorLocation` _mainmenucamera)))
  ;[1 1 1] On any key pressed, start transition to tutorial level
  (:`Pressed`
    (`/Engine/EditorBlueprintResources/StandardMacros.DoOnce` false
      (:`Completed`
        (`/Game/MyContent/Blueprints/Widgets/UMG_MainMenu.StartMainMenuTransition` (`self.MainMenuHUD`))
        (`self.K2_DestroyActor` (`self.TitleSmoke`))
        ;[1 1 1] Possible to replace with level sequencer
        (bind (_direction _alpha) (`Timeline|CameraTransitionTimeline`)
          (:`Update`
            ;;[1 1 1] Move camera for initial height to final height over time
            (`self.K2_SetActorLocation` _mainmenucamera (`KismetMathLibrary.MakeVector` _returnvalue_x _returnvalue_y (`KismetMathLibrary.Lerp` (`self.CameraInitialHeight`) (`self.CameraFinalHeight`) _alpha)) false false)))))))

(fn `UserConstructionScript`)