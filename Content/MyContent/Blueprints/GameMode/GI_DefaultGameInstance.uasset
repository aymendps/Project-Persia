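; Game instance that carries player state between levels.
; SavePlayerPersistentData copies max health, current health and sword ownership from the player's Health and PlayerWeaponManager components into instance variables, storing full health if the player died.
; RetrievePlayerPersistentData writes those stored values back onto a given player character.
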(fn `RetrievePlayerPersistentData`
  (params (OutPlayerCharacter :type "/Game/MyContent/Blueprints/Characters/Player/BP_PlayerCharacter Object Reference (by ref)"))
  (bind _health (`/Game/MyContent/Blueprints/Characters/Player/BP_PlayerCharacter.Health` OutPlayerCharacter))
  (`|ExecutionSequence`
    (:`then_0`
      ;[1 1 1] Retrieve health related data
      (set `HealthComponent.MaxHealth` (`self.PlayerMaxHealth`) _health)
      (set `HealthComponent.CurrentHealth` (`self.PlayerHealth`) _health))
    (:`then_1`
      ;[1 1 1] Retrieve fighting related data
      (set `/Game/MyContent/Blueprints/Components/AC_PlayerWeaponManager.HasSword` (`self.PlayerHasSword`) (`/Game/MyContent/Blueprints/Characters/Player/BP_PlayerCharacter.PlayerWeaponManager` OutPlayerCharacter)))))

(fn `SavePlayerPersistentData`
  (params (PlayerCharacter :type "/Game/MyContent/Blueprints/Characters/Player/BP_PlayerCharacter Object Reference"))
  (bind _health (`/Game/MyContent/Blueprints/Characters/Player/BP_PlayerCharacter.Health` PlayerCharacter))
  (bind _currenthealth (`HealthComponent.CurrentHealth` _health))
  (`|ExecutionSequence`
    (:`then_0`
      ;[1 1 1] Save health related data
      (bind _output_get (set `self.PlayerMaxHealth` (`HealthComponent.MaxHealth` _health)))
      ;;[1 1 1] If the player died this level, reset current health to max health so that the player starts healthy when loading the next level.
      ;; Otherwise, keep the current health as it is.
      (set `self.PlayerHealth` (`KismetMathLibrary.SelectFloat` _output_get _currenthealth (<= _currenthealth 0.0))))
    (:`then_1`
      ;[1 1 1] Save fight related data
      (set `self.PlayerHasSword` (`/Game/MyContent/Blueprints/Components/AC_PlayerWeaponManager.HasSword` (`/Game/MyContent/Blueprints/Characters/Player/BP_PlayerCharacter.PlayerWeaponManager` PlayerCharacter))))))