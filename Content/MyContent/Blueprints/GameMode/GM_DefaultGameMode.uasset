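; Default game mode that handles level transitions and carries player state between levels.
; On BeginPlay it restores persistent player data from the game instance and starts persistent level music.
; LoadLevel replaces direct OpenLevel calls: it hides the HUD, stops camera follow, fades out, then optionally saves player data before opening the level.
; RestartThisLevel, meant for player death, reloads the current level through LoadLevel without saving.
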(event `self.ReceiveBeginPlay`
  (set `self.PlayerCharacter` (cast `/Game/MyContent/Blueprints/Characters/Player/BP_PlayerCharacter` (`GameplayStatics.GetPlayerCharacter` 0) :!pure true))
  (bind _output_get (set `self.GameInstance` (cast `/Game/MyContent/Blueprints/GameMode/GI_DefaultGameInstance` (`GameplayStatics.GetGameInstance`) :!pure true)))
  (`/Game/MyContent/Blueprints/GameMode/GI_DefaultGameInstance.RetrievePlayerPersistentData` _output_get (`self.PlayerCharacter`))
  (`/Game/MyContent/Blueprints/GameMode/GI_DefaultGameInstance.PlayPersistentLevelMusic` (`self.GameInstance`)))

(event `Event LoadLevel`
  (params (LevelToLoad :type Name) (`SavePlayerData?` :type Boolean :default true))
  (bind _playercharacter (`self.PlayerCharacter`))
  (bind _playercameramanager (`/Game/MyContent/Blueprints/Characters/Player/BP_PlayerCharacter.PlayerCameraManager` _playercharacter))
  ;[1 1 1] LoadLevel - Call when loading a level instead of OpenLevel to play fade out sequence and save player's persistent data
  (`/Game/MyContent/Blueprints/GameMode/BP_PlayerController.HidePlayerHUD` (`/Game/MyContent/Blueprints/Characters/Player/BP_PlayerCharacter.PlayerController` _playercharacter))
  (set `/Game/MyContent/Blueprints/Cameras/BP_PlayerCameraManager.ShouldFollowTarget` false _playercameramanager)
  (`/Game/MyContent/Blueprints/Cameras/BP_PlayerCameraManager.FadeOutCamera` _playercameramanager)
  ;;[1 1 1] Wait for fade out to end
  (`KismetSystemLibrary.Delay` 2.0)
  (if `SavePlayerData?`
    ;;[1 1 1] Save player persistent data to be retrieved in next level
    (`/Game/MyContent/Blueprints/GameMode/GI_DefaultGameInstance.SavePlayerPersistentData` (`self.GameInstance`) (`self.PlayerCharacter`)))
  (`GameplayStatics.OpenLevel` LevelToLoad))

(event `Event RestartThisLevel`
  ;[1 1 1] RestartThisLevel - Call when a player dies to restart this level
  (bind _returnvalue (`GameplayStatics.GetCurrentLevelName` true))
  (`self.Event LoadLevel` (`KismetStringLibrary.Conv_StringToName` _returnvalue) false))

(fn `UserConstructionScript`)