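; Level exit stairs that, once unlocked, let the player interact to climb them and travel to another level.
; UnlockStairs triggers the child-actor door, then marks the stairs unlocked after a short delay so the player avoids the moving door.
; Interact disables input, clears the movement plane constraint, and navmesh-moves the player to a destination.
; The camera stops following and fades out before the configured level loads.
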(event `self.ReceiveBeginPlay`
  ;[1 1 1] Cache a reference to BP of the door, which is a child component of this
  (set `self.BPLevelStairsDoor` (cast `/Game/MyContent/Blueprints/Doors/BP_LevelStairsDoor` (`ChildActorComponent.ChildActor` (`self.Door`)) :!pure true)))

(event `UnlockStairs`
  ;[1 1 1] Trigger the door so that it opens/closes then set this to unlocked after a small delay to avoid the player running into the door when it's still moving
  (if (not (`self.isUnlocked`))
    (`/Game/MyContent/Blueprints/Doors/BP_LevelStairsDoor.Door Trigger Activated` (`self.BPLevelStairsDoor`))
    (`KismetSystemLibrary.Delay` 0.6)
    (set `self.isUnlocked` true)))

(event `self.Interact`
  (params (PlayerCharacter :type "PlayerCharacter Object Reference"))
  (bind _asbp_player_character (cast `/Game/MyContent/Blueprints/Characters/Player/BP_PlayerCharacter` PlayerCharacter :!pure true))
  (bind _playercameramanager (`/Game/MyContent/Blueprints/Characters/Player/BP_PlayerCharacter.PlayerCameraManager` _asbp_player_character))
  ;[1 1 1] Interact (From Interface) Implementation - Called when the player triggers the interact input and the stairs are unlocked
  (if (`self.isUnlocked`)
    ;;[1 1 1] Disable player input and remove the plain constraint so the character can go up the stairs
    (`self.DisableInput` _asbp_player_character null)
    (`MovementComponent.SetPlaneConstraintNormal` (`Character.CharacterMovement` _asbp_player_character) (0.0 0.0 0.0))
    ;;[1 1 1] Move the player up the stairs using the navmesh
    (`AIBlueprintHelperLibrary.SimpleMoveToLocation` (`GameplayStatics.GetPlayerController` 0) (`SceneComponent.K2_GetComponentLocation` (`self.PlayerDestination`)))
    (set `/Game/MyContent/Blueprints/Cameras/BP_PlayerCameraManager.ShouldFollowTarget` false _playercameramanager)
    (`/Game/MyContent/Blueprints/Cameras/BP_PlayerCameraManager.FadeOutCamera` _playercameramanager)
    (`KismetSystemLibrary.Delay` (`self.DelayBeforeOpeningLevel`))
    (`GameplayStatics.OpenLevel` (`self.LevelToLoad`))))

(fn `UserConstructionScript`)