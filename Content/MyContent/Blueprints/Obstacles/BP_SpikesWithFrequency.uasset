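; Spike obstacle that repeatedly rises and retracts on a timed cycle.
; After an initial delay on BeginPlay, an Appear timeline and a Disappear timeline alternately drive MoveSpikesSmoothly, with configurable waits after each phase.
; The sequence loops by re-invoking its own BeginSpikesSequence event when retraction ends.
; The construction script calls the parent's, then sets both timeline play rates from the appear and disappear speed variables.
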(event `self.ReceiveBeginPlay`
  ;[1 1 1] Start Spikes Sequence
  (`KismetSystemLibrary.Delay` (`self.DelayBeforeSequence`))
  (`self.BeginSpikesSequence`))

(event `BeginSpikesSequence`
  ;[1 1 1] Spikes appear over time
  (bind (_direction _appear) (`Timeline|Appear Timeline` :!via `PlayFromStart`)
    (:`Update`
      (`self.MoveSpikesSmoothly` _appear))
    (:`Finished`
      ;[1 1 1] Wait for some time after spikes appear
      (`KismetSystemLibrary.Delay` (`self.DelayAfterAppear`))
      ;[1 1 1] Spikes disappear over time
      (bind (_direction_2 _disappear) (`Timeline|Disappear Timeline` :!via `PlayFromStart`)
        (:`Update`
          (`self.MoveSpikesSmoothly` _disappear))
        (:`Finished`
          ;[1 1 1] Wait for some time after spikes disappear, then invoke this event once more
          (`KismetSystemLibrary.Delay` (`self.DelayAfterDisappear`))
          (`self.BeginSpikesSequence`))))))

(fn `UserConstructionScript`
  ;[1 1 1] Set timelines' play rate
  (`parent.UserConstructionScript`)
  (`TimelineComponent.SetPlayRate` (`self.Appear Timeline`) (`self.SpikesAppearSpeed`))
  (`TimelineComponent.SetPlayRate` (`self.Disappear Timeline`) (`self.SpikesDisappearSpeed`)))