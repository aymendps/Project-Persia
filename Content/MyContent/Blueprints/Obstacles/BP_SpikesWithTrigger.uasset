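; Spike trap obstacle that raises its spikes when something overlaps its trigger sphere and lowers them when the overlap ends.
; Appear and Disappear timelines drive MoveSpikesSmoothly; the cached Disappear alpha sets the Appear start time to avoid snapping on re-entry.
; The construction script applies the configurable trigger radius and both timeline play rates.
; Spike hits only print a placeholder message, with no damage applied.
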(event `self.TriggerSphere.OnComponentBeginOverlap`
  (params (OverlappedComponent :type "PrimitiveComponent Object Reference") (OtherActor :type "Actor Object Reference") (OtherComp :type "PrimitiveComponent Object Reference") (OtherBodyIndex :type Integer) (bFromSweep :type Boolean) (SweepResult :type "HitResult Structure (by ref)"))
  ;[1 1 1] Spikes appear when player enters trigger sphere
  ;;[1 1 1] Stop the Disappear timeline so it does not interfere with this one
  (`TimelineComponent.Stop` (`self.Disappear Timeline`))
  ;;[1 1 1] Use the time that the Disappear timeline stopped so that the spikes don't snap to the initial location
  (`TimelineComponent.SetNewTime` (`self.Appear Timeline`) (`self.DisappearAlpha`))
  ;;[1 1 1] Move the spikes upwards over time
  (bind (_direction _appear) (`Timeline|Appear Timeline`)
    (:`Update`
      (`self.MoveSpikesSmoothly` _appear))))

(event `self.TriggerSphere.OnComponentEndOverlap`
  (params (OverlappedComponent :type "PrimitiveComponent Object Reference") (OtherActor :type "Actor Object Reference") (OtherComp :type "PrimitiveComponent Object Reference") (OtherBodyIndex :type Integer))
  ;[1 1 1] Spikes disappear when the player leaves the trigger sphere
  ;;[1 1 1] Move the spikes downwards over time and cache the value of the alpha
  (bind (_direction _disappear) (`Timeline|Disappear Timeline` :!via `PlayFromStart`)
    (:`Update`
      (bind _output_get (set `self.DisappearAlpha` _disappear))
      (`self.MoveSpikesSmoothly` _output_get))))

(event `self.SM_Spikes.OnComponentHit`
  (params (HitComponent :type "PrimitiveComponent Object Reference") (OtherActor :type "Actor Object Reference") (OtherComp :type "PrimitiveComponent Object Reference") (NormalImpulse :type "Vector Structure") (Hit :type "HitResult Structure (by ref)"))
  (`KismetSystemLibrary.PrintString` "Player should take damage or die" true true (struct :`R` 1.0 :`A` 1.0)))

(fn `UserConstructionScript`
  ;[1 1 1] Set the trigger sphere radius and the play rate of the timelines
  (`parent.UserConstructionScript`)
  (`SphereComponent.SetSphereRadius` (`self.TriggerSphere`) (`self.TriggerRadius`) false)
  (`TimelineComponent.SetPlayRate` (`self.Appear Timeline`) (`self.SpikesAppearSpeed`))
  (`TimelineComponent.SetPlayRate` (`self.Disappear Timeline`) (`self.SpikesDisappearSpeed`)))