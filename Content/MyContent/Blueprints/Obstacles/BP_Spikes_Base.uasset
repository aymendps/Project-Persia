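; Base Blueprint for a spike obstacle that can rise along Z and detects overlaps with the player character.
; The construction script caches the spike mesh's starting relative Z and an end Z offset by SpikesGoUpByZ.
; MoveSpikesSmoothly lerps the mesh between those heights from an alpha meant to come from a timeline, which this file does not contain.
; Player overlap only prints a placeholder message, with no damage or death applied.
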(event `self.SM_Spikes.OnComponentBeginOverlap`
  (params (OverlappedComponent :type "PrimitiveComponent Object Reference") (OtherActor :type "Actor Object Reference") (OtherComp :type "PrimitiveComponent Object Reference") (OtherBodyIndex :type Integer) (bFromSweep :type Boolean) (SweepResult :type "HitResult Structure (by ref)"))
  (cast `/Game/MyContent/Blueprints/Characters/Player/BP_PlayerCharacter` OtherActor)
  (`KismetSystemLibrary.PrintString` "Player should die or take damage" true true (struct :`R` 1.0 :`A` 1.0)))

(fn `MoveSpikesSmoothly`
  (params (`Lerp Alpha` :type "Float (double-precision)"))
  (bind _sm_spikes (`self.SM_Spikes`))
  (bind (_relativelocation_x _relativelocation_y) (`KismetMathLibrary.BreakVector` (`SceneComponent.RelativeLocation` _sm_spikes)))
  ;[1 1 1] Lerp between the initial and final Z position using the timeline's alpha and update the spikes' location
  (`SceneComponent.K2_SetRelativeLocation` _sm_spikes (`KismetMathLibrary.MakeVector` _relativelocation_x _relativelocation_y (`KismetMathLibrary.Lerp` (`self.InitialSpikesZPos`) (`self.FinalSpikesZPos`) `Lerp Alpha`)) false false))

(fn `UserConstructionScript`
  (bind (_relativelocation_x _relativelocation_y _relativelocation_z) (`KismetMathLibrary.BreakVector` (`SceneComponent.RelativeLocation` (`self.SM_Spikes`))))
  ;[1 1 1] Set the initial and final Z position of the spikes to move from/to
  (bind _output_get (set `self.InitialSpikesZPos` _relativelocation_z))
  (set `self.FinalSpikesZPos` (+ _output_get (`self.SpikesGoUpByZ`))))