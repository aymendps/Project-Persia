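; Timed cell door that slides vertically when the player steps on its pressure plate, then returns after a delay once the plate is vacated.
; Construction script derives start and target positions from mesh bounds and StartsOpen, shows a direction arrow and sets both timeline speeds.
; Separate activate and timeout timelines lerp the door, with LastAlpha letting activation interrupt a return mid-travel.
; Plate movement and door audio accompany each transition.
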(event `self.DoorTrigger.OnComponentBeginOverlap`
  (params (OverlappedComponent :type "PrimitiveComponent Object Reference") (OtherActor :type "Actor Object Reference") (OtherComp :type "PrimitiveComponent Object Reference") (OtherBodyIndex :type Integer) (bFromSweep :type Boolean) (SweepResult :type "HitResult Structure (by ref)"))
  ;[1 1 1] Flag the trigger as activated and only call DoorTriggerActivated event if the door is completely open/closed
  (cast `/Game/MyContent/Blueprints/Characters/Player/BP_PlayerCharacter` OtherActor)
  (set `self.IsActivated` true)
  (if (not (`TimelineComponent.IsPlaying` (`self.Trigger Activated Timeline`)))
    ;;[1 1 1] If Last Alpha equals 1, that means that the door did not time out yet, so we don't need to activate it again just yet
    (if (!= (`self.LastAlpha`) 1.0)
      (`self.DoorTriggerActivated`))))

(event `self.DoorTrigger.OnComponentEndOverlap`
  (params (OverlappedComponent :type "PrimitiveComponent Object Reference") (OtherActor :type "Actor Object Reference") (OtherComp :type "PrimitiveComponent Object Reference") (OtherBodyIndex :type Integer))
  ;[1 1 1] Flag the trigger as deactivated and only call InvokeDoorTriggerTimedOut if the door is completely open/closed
  (cast `/Game/MyContent/Blueprints/Characters/Player/BP_PlayerCharacter` OtherActor)
  (set `self.IsActivated` false)
  (if (not (`TimelineComponent.IsPlaying` (`self.Trigger Activated Timeline`)))
    (`self.InvokeDoorTriggerTimedOut`)))

(event `DoorTriggerActivated`
  ;[1 1 1] DoorTriggerActivated event - Called when the player enters the pressure plate's trigger if this is not being executed already
  ;;[1 1 1] Move presure plate downwards to represent it being pressed
  (`self.MovePressurePlate` (`self.Pressure Plate`))
  (`self.PlayDoorAudio`)
  ;;[1 1 1] Stop the timed out timeline and continue from where the door stopped: Move the door over time from that point and then call InvokeDoorTriggerTimedOut once it's fully open/closed
  (`TimelineComponent.Stop` (`self.Timed Out Timeline`))
  (`TimelineComponent.SetNewTime` (`self.Trigger Activated Timeline`) (`self.LastAlpha`))
  (bind (_direction _lerp_alpha) (`Timeline|Trigger Activated Timeline`)
    (:`Update`
      (bind _output_get (set `self.LastAlpha` _lerp_alpha))
      (`self.MoveDoorSmoothly` _output_get))
    (:`Finished`
      (`self.StopDoorAudio`)
      (`self.InvokeDoorTriggerTimedOut`))))

(event `DoorTriggerTimedOut`
  ;[1 1 1] DoorTriggerTimedOut event - Called when the player leave the pressure plate's trigger after a certain delay if this is being executed already
  ;;[1 1 1] Move pressure plate upwards to represent it being released
  (`self.MovePressurePlate` (`self.Pressure Plate`) true)
  (`self.PlayDoorAudio`)
  ;;[1 1 1] Open/Close the door over time
  (bind (_direction _lerp_alpha) (`Timeline|Timed Out Timeline` :!via `PlayFromStart`)
    (:`Update`
      (bind _output_get (set `self.LastAlpha` _lerp_alpha))
      (`self.MoveDoorSmoothly` _output_get))
    (:`Finished`
      (`self.StopDoorAudio`))))

(fn `CalculateDoorHeight`
  (bind (_min _max) (`StaticMeshComponent.GetLocalBounds` (`self.SM_Cell_Door`)))
  ;[1 1 1] Subtract the bottom bound from the top bound to get the door height. Then add the height offset before setting its value
  (set `self.DoorHeight` (+ (`self.DoorHeightOffset`) (- (.z _max) (.z _min)))))

(fn `CalculateDoorInitialLocation`
  (bind (_relativelocation_x _relativelocation_y _relativelocation_z) (`KismetMathLibrary.BreakVector` (`SceneComponent.RelativeLocation` (`self.SM_Cell_Door`))))
  ;[1 1 1] If the door starts open, then update its relative location so it becomes open.
  (if (`self.StartsOpen`)
    ;[1 1 1] Move the door's relative location upwards instantly using the door height, so that it starts open
    (bind _output_get (set `self.DoorInitialLocation` (`KismetMathLibrary.MakeVector` _relativelocation_x _relativelocation_y (+ _relativelocation_z (`self.DoorHeight`)))))
    (`SceneComponent.K2_SetRelativeLocation` (`self.SM_Cell_Door`) _output_get false false)
    (else
      ;[1 1 1] Just set the value of initial location to the current relative location since the door starts closed, which is the default state
      (set `self.DoorInitialLocation` (`SceneComponent.RelativeLocation` (`self.SM_Cell_Door`))))))

(fn `CalculateDoorTargetLocation`
  (bind (_relativelocation_x _relativelocation_y _relativelocation_z) (`KismetMathLibrary.BreakVector` (`SceneComponent.RelativeLocation` (`self.SM_Cell_Door`))))
  ;[1 1 1] If the door is initially open, multiply the door's height by -1 so that adding it with the door's relative location will result in subtracting it instead, otherwise keep the value of the door height as is. This will result in finding the correct target location depending on if the door is going to open or close.
  (set `self.DoorTargetLocation` (`KismetMathLibrary.MakeVector` _relativelocation_x _relativelocation_y (+ _relativelocation_z (`KismetMathLibrary.SelectFloat` (* (`self.DoorHeight`) -1.0) (`self.DoorHeight`) (`self.StartsOpen`))))))

(fn `MoveDoorSmoothly`
  (params (Alpha :type "Float (single-precision)"))
  ;[1 1 1] Use the timeline alpha to lerp from the initial location to the target location, then using the result to move the relative location of the door
  (`SceneComponent.K2_SetRelativeLocation` (`self.SM_Cell_Door`) (`KismetMathLibrary.VLerp` (`self.DoorInitialLocation`) (`self.DoorTargetLocation`) Alpha) false false))

(fn `MovePressurePlate`
  (params (`Pressure Plate` :type "SceneComponent Object Reference") (Upwards :type Boolean))
  (bind (_relativelocation_x _relativelocation_y _relativelocation_z) (`KismetMathLibrary.BreakVector` (`SceneComponent.RelativeLocation` `Pressure Plate`)))
  (bind _platesgodownbyz (`self.PlatesGoDownByZ`))
  (`SceneComponent.K2_SetRelativeLocation` `Pressure Plate` (`KismetMathLibrary.MakeVector` _relativelocation_x _relativelocation_y (- _relativelocation_z (`KismetMathLibrary.SelectFloat` (* -1.0 _platesgodownbyz) _platesgodownbyz Upwards))) false false))

(fn `PlayDoorAudio`
  (bind _dooraudiocomponent (`self.DoorAudioComponent`)
    (:`then`
      (if (not (`AudioComponent.IsPlaying` _dooraudiocomponent))
        (`AudioComponent.Play` _dooraudiocomponent 0.0)))
    (:`else`
      (bind _returnvalue (`GameplayStatics.SpawnSoundAtLocation` "/Game/MyContent/Audio/A_DoorMoving.A_DoorMoving" (`self.K2_GetActorLocation`) (struct) 1.0 1.0 0.0 null null false))
      (set `self.DoorAudioComponent` _returnvalue))))

(fn `ShowDoorDirectionArrow`
  ;[1 1 1] Show the Opening Arrow if the door starts closed. Show the Closing Arrow if the door starts open
  (`SceneComponent.SetVisibility` (`self.Closing Arrow`) (`self.StartsOpen`) false)
  (`SceneComponent.SetVisibility` (`self.Opening Arrow`) (not (`self.StartsOpen`)) false))

(fn `StopDoorAudio`
  (bind _dooraudiocomponent (`self.DoorAudioComponent`)
    (:`then`
      (`AudioComponent.StopDelayed` _dooraudiocomponent 0.3)
      (`GameplayStatics.PlaySoundAtLocation` "/Game/MyContent/Audio/A_DoorStopped.A_DoorStopped" (`self.K2_GetActorLocation`) (struct) 1.0 1.0 0.0 null null null null))
    (:`else`)))

(fn `UserConstructionScript`
  ;[1 1 1] Initialize door depending on chosen settings
  (`self.ShowDoorDirectionArrow`)
  (`self.CalculateDoorHeight`)
  (`self.CalculateDoorInitialLocation`)
  (`self.CalculateDoorTargetLocation`)
  (`TimelineComponent.SetPlayRate` (`self.Trigger Activated Timeline`) (`self.NormalDoorSpeed`))
  (`TimelineComponent.SetPlayRate` (`self.Timed Out Timeline`) (`self.TimedOutDoorSpeed`)))