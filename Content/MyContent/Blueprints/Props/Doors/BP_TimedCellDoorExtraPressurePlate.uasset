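; Timed cell door variant, built on a parent door Blueprint, that adds an extra pressure plate the player character can stand on to trigger it.
; Overlapping the plate's trigger activates the door unless it is mid-activation or has not timed out; leaving starts a delayed time-out, skipped if the plate is reoccupied.
; Activation and time-out events press or release the plate, then call the parent's door logic.
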(event `self.Extra DoorTrigger.OnComponentBeginOverlap`
  (params (OverlappedComponent :type "PrimitiveComponent Object Reference") (OtherActor :type "Actor Object Reference") (OtherComp :type "PrimitiveComponent Object Reference") (OtherBodyIndex :type Integer) (bFromSweep :type Boolean) (SweepResult :type "HitResult Structure (by ref)"))
  ;[1 1 1] Flag the trigger as activated and only call DoorTriggerActivated event if the door is completely open/closed
  (cast `/Game/MyContent/Blueprints/Characters/Player/BP_PlayerCharacter` OtherActor)
  (set `self.IsActivated` true)
  (if (not (`TimelineComponent.IsPlaying` (`self.Trigger Activated Timeline`)))
    ;;[1 1 1] If Last Alpha equals 1, that means that the door did not time out yet, so we don't need to activate it again just yet
    (if (!= (`self.LastAlpha`) 1.0)
      (`self.DoorTriggerActivated`))))

(event `self.Extra DoorTrigger.OnComponentEndOverlap`
  (params (OverlappedComponent :type "PrimitiveComponent Object Reference") (OtherActor :type "Actor Object Reference") (OtherComp :type "PrimitiveComponent Object Reference") (OtherBodyIndex :type Integer))
  ;[1 1 1] Flag the trigger as deactivated and only call InvokeDoorTriggerTimedOut if the door is completely open/closed
  (cast `/Game/MyContent/Blueprints/Characters/Player/BP_PlayerCharacter` OtherActor)
  (set `self.IsActivated` false)
  (if (not (`TimelineComponent.IsPlaying` (`self.Trigger Activated Timeline`)))
    (`self.InvokeDoorTriggerTimedOut`)))

(event `self.DoorTriggerActivated`
  ;[1 1 1] Move extra presure plate downwards to represent it being pressed
  (`self.MovePressurePlate` (`self.Extra Pressure Plate`))
  (`parent.DoorTriggerActivated`))

(event `self.DoorTriggerTimedOut`
  ;[1 1 1] Move extra presure plate upwards to represent it being released
  (`self.MovePressurePlate` (`self.Extra Pressure Plate`) true)
  (`parent.DoorTriggerTimedOut`))

(fn `UserConstructionScript`
  (`parent.UserConstructionScript`))