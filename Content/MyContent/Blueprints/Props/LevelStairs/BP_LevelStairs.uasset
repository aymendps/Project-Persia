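; Level stairs prop that, once unlocked, lets the player walk up it to leave for another level.
; Unlocking triggers the child-actor door and enables interaction.
; Interacting disables player input, clears the movement plane constraint, and auto-walks the character to a destination point via navmesh.
; The game mode's level-load event fires as the walk starts, using the stairs' target level.
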(event `self.ReceiveBeginPlay`
  ;[1 1 1] Cache a reference to BP of the door, which is a child component of this
  (set `self.BPLevelStairsDoor` (cast `/Game/MyContent/Blueprints/Props/Doors/BP_LevelStairsDoor` (`ChildActorComponent.ChildActor` (`self.Door`)) :!pure true)))

(event `UnlockStairs`
  ;[1 1 1] Trigger the door so that it opens/closes then allow player interaction
  (if (not (`self.CanInteractWithThis`))
    (`/Game/MyContent/Blueprints/Props/Doors/BP_LevelStairsDoor.Door Trigger Activated` (`self.BPLevelStairsDoor`))
    (set `self.CanInteractWithThis` true)))

(event `self.Interact`
  (params (PlayerCharacter :type "PlayerCharacter Object Reference"))
  ;[1 1 1] Interact (From Interface) Implementation - Called when the player triggers the interact input and the stairs are unlocked
  (if (`self.CanInteractWithThis`)
    ;;[1 1 1] Disable player input and remove the plain constraint so the character can go up the stairs
    (set `/Game/MyContent/Blueprints/Characters/Player/BP_PlayerController.bEnableInput` false (cast `/Game/MyContent/Blueprints/Characters/Player/BP_PlayerController` (`GameplayStatics.GetPlayerController` 0) :!pure true))
    (`MovementComponent.SetPlaneConstraintNormal` (`Character.CharacterMovement` PlayerCharacter) (0.0 0.0 0.0))
    ;;[1 1 1] Move the player up the stairs using the navmesh
    (`AIBlueprintHelperLibrary.SimpleMoveToLocation` (`GameplayStatics.GetPlayerController` 0) (`SceneComponent.K2_GetComponentLocation` (`self.PlayerDestination`)))
    (`/Game/MyContent/Blueprints/GameMode/BP_DefaultGameMode.Event LoadLevel` (cast `/Game/MyContent/Blueprints/GameMode/BP_DefaultGameMode` (`GameplayStatics.GetGameMode`) :!pure true) (`self.LevelToLoad`))))

(fn `UserConstructionScript`)