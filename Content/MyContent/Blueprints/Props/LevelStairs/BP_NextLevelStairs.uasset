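; Level-exit stairs prop that takes the player to the next level on interaction.
; A player entering the box reveals the button indicator and unlocks the stairs, triggering the child-actor door once.
; Interacting clears the movement plane constraint, walks the player to the destination via navmesh, and has the game mode load the configured level, saving player data.
; Interaction while locked just ends after a short delay for the camera zoom.
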(event `self.ReceiveBeginPlay`
  ;[1 1 1] Cache a reference to BP of the door, which is a child component of this
  (set `self.BPLevelStairsDoor` (cast `/Game/MyContent/Blueprints/Props/Doors/BP_LevelStairsDoor` (`ChildActorComponent.ChildActor` (`self.Door`)) :!pure true)))

(event `self.Box.OnComponentBeginOverlap`
  (params (OverlappedComponent :type "PrimitiveComponent Object Reference") (OtherActor :type "Actor Object Reference") (OtherComp :type "PrimitiveComponent Object Reference") (OtherBodyIndex :type Integer) (bFromSweep :type Boolean) (SweepResult :type "HitResult Structure (by ref)"))
  (cast `/Game/MyContent/Blueprints/Characters/Player/BP_PlayerCharacter` OtherActor)
  ;[1 1 1] Display button indicator since player can interact with this now
  (`SceneComponent.SetVisibility` (`self.Interact Button Indicator`) true false)
  (`self.UnlockStairs`))

(event `UnlockStairs`
  ;[1 1 1] Trigger the door so that it opens/closes then allow player interaction
  (if (not (`self.CanInteractWithThis`))
    (`/Game/MyContent/Blueprints/Props/Doors/BP_LevelStairsDoor.Door Trigger Activated` (`self.BPLevelStairsDoor`))
    (set `self.CanInteractWithThis` true)))

(event `self.Interact`
  (params (PlayerCharacter :type "PlayerCharacter Object Reference"))
  ;[1 1 1] Interact (From Interface) Implementation - Called when the player triggers the interact input and the stairs are unlocked
  (if (`self.CanInteractWithThis`)
    ;;[1 1 1] Hide button indicator since player interacted
    (`SceneComponent.SetVisibility` (`self.Interact Button Indicator`) false false)
    (`MovementComponent.SetPlaneConstraintNormal` (`Character.CharacterMovement` PlayerCharacter) (0.0 0.0 0.0))
    ;;[1 1 1] Move the player up the stairs using the navmesh
    (`AIBlueprintHelperLibrary.SimpleMoveToLocation` (`GameplayStatics.GetPlayerController` 0) (`SceneComponent.K2_GetComponentLocation` (`self.PlayerDestination`)))
    (`/Game/MyContent/Blueprints/GameMode/GM_DefaultGameMode.Event LoadLevel` (cast `/Game/MyContent/Blueprints/GameMode/GM_DefaultGameMode` (`GameplayStatics.GetGameMode`) :!pure true) (`self.LevelToLoad`) true)
    (else
      ;;[1 1 1] In case something unexpected happens and the player interacts with this when it's not possible, wait for a small delay to let the camera zoom in when interacting, then call finished interact event without taking any other action.
      (`KismetSystemLibrary.Delay` 1.0)
      (`/Game/MyContent/Blueprints/GameMode/BP_PlayerController.Event FinishedInteract` (cast `/Game/MyContent/Blueprints/GameMode/BP_PlayerController` (`GameplayStatics.GetPlayerController` 0) :!pure true) false))))

(fn `UserConstructionScript`)