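; Stairs prop with a child-actor door that plays a level intro, walking the player down from the previous level.
; On BeginPlay, if enabled, it disables input and camera follow, lifts the plane constraint and nav-moves the player from StartPoint to DestinationPoint.
; Timed delays close the door, then snap the player to a hardcoded Y and restore single-axis movement, camera and input.
; With the intro disabled, it only triggers the door.
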(event `self.ReceiveBeginPlay`
  ;[1 1 1] Cache a reference to BP of the door, which is a child component of this, and the player character to be used
  (set `self.BPLevelStairsDoor` (cast `/Game/MyContent/Blueprints/Props/Doors/BP_LevelStairsDoor` (`ChildActorComponent.ChildActor` (`self.Door`)) :!pure true))
  (set `self.PlayerCharacter` (cast `/Game/MyContent/Blueprints/Characters/Player/BP_PlayerCharacter` (`GameplayStatics.GetPlayerCharacter` 0) :!pure true))
  ;[1 1 1] Wait a small delay for everything to initialize then start level intro animation
  (`KismetSystemLibrary.Delay` 0.1)
  (`self.LevelIntroAnimation`))

(event `LevelIntroAnimation`
  (bind _playercharacter (`self.PlayerCharacter`))
  (bind _playercharacter_2 (`self.PlayerCharacter`))
  (bind (_returnvalue_x _returnvalue_y _returnvalue_z) (`KismetMathLibrary.BreakVector` (`self.K2_GetActorLocation` _playercharacter)))
  (if (`self.RunIntroAnimation?`)
    (`self.WalkPlayerDownStairs`)
    ;[1 1 1] Wait for the player to reach a certain point in stairs and then start closing door
    (`KismetSystemLibrary.Delay` 1.0)
    (`/Game/MyContent/Blueprints/Props/Doors/BP_LevelStairsDoor.Door Trigger Activated` (`self.BPLevelStairsDoor`))
    ;[1 1 1] Wait for player to reach the destination point and then fix the position in case that the navigation stopped a bit earlier than expected
    (`KismetSystemLibrary.Delay` 1.0)
    (`self.K2_SetActorLocation` _playercharacter (`KismetMathLibrary.MakeVector` _returnvalue_x -720.0 _returnvalue_z) false false)
    ;[1 1 1] Restore normal constraint so player moves on one axis as they should
    (`MovementComponent.SetPlaneConstraintNormal` (`Character.CharacterMovement` (`self.PlayerCharacter`)) (0.0 1.0 0.0))
    (set `/Game/MyContent/Blueprints/Cameras/BP_PlayerCameraManager.ShouldFollowTarget` true (`/Game/MyContent/Blueprints/Characters/Player/BP_PlayerCharacter.PlayerCameraManager` _playercharacter_2))
    (set `/Game/MyContent/Blueprints/GameMode/BP_PlayerController.bEnableInput` true (`/Game/MyContent/Blueprints/Characters/Player/BP_PlayerCharacter.PlayerController` _playercharacter_2))
    (else
      ;[1 1 1] If we don't need to walk player down the stairs, just close the door and move on
      (`/Game/MyContent/Blueprints/Props/Doors/BP_LevelStairsDoor.Door Trigger Activated` (`self.BPLevelStairsDoor`)))))

(fn `UserConstructionScript`)

(fn `WalkPlayerDownStairs`
  (bind _playercharacter (`self.PlayerCharacter`))
  ;[1 1 1] Disable input and camera following until the player walks down the stairs successfully
  (set `/Game/MyContent/Blueprints/Cameras/BP_PlayerCameraManager.ShouldFollowTarget` false (`/Game/MyContent/Blueprints/Characters/Player/BP_PlayerCharacter.PlayerCameraManager` _playercharacter))
  (set `/Game/MyContent/Blueprints/GameMode/BP_PlayerController.bEnableInput` false (`/Game/MyContent/Blueprints/Characters/Player/BP_PlayerCharacter.PlayerController` _playercharacter))
  ;[1 1 1] Remove plane constraint to allow controller to use nav mesh
  (`MovementComponent.SetPlaneConstraintNormal` (`Character.CharacterMovement` (`self.PlayerCharacter`)) (0.0 0.0 0.0))
  ;[1 1 1] Teleport player to start point
  (`self.K2_SetActorLocation` (`self.PlayerCharacter`) (`SceneComponent.K2_GetComponentLocation` (`self.StartPoint`)) false false)
  ;[1 1 1] Walk down stairs
  (`AIBlueprintHelperLibrary.SimpleMoveToLocation` (`/Game/MyContent/Blueprints/Characters/Player/BP_PlayerCharacter.PlayerController` (`self.PlayerCharacter`)) (`SceneComponent.K2_GetComponentLocation` (`self.DestinationPoint`))))