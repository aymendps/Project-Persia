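; BP_SpikesPermanent is an always-active spike obstacle prop that damages the player character on contact.
; It caches the player character on BeginPlay, then checks every Tick whether the SMSpikes mesh overlaps that character.
; Slow walking makes the player immune; otherwise it applies SpikesDamage with the BP_DamageType_Spikes damage type on each overlapping frame.
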(event `self.ReceiveBeginPlay`
  ;[1 1 1] Get reference to player
  (set `self.PlayerCharacter` (cast `/Game/MyContent/Blueprints/Characters/Player/BP_PlayerCharacter` (`GameplayStatics.GetPlayerCharacter` 0) :!pure true)))

(event `self.ReceiveTick`
  (params (DeltaSeconds :type "Float (single-precision)"))
  ;[1 1 1] Damage player if possible
  (if (`self.CanDamagePlayerCharacter`)
    (`GameplayStatics.ApplyDamage` (`self.PlayerCharacter`) (`self.Spikes Damage`) null self "/Game/MyContent/Blueprints/DamageTypes/BP_DamageType_Spikes.BP_DamageType_Spikes_C")))

(fn `CanDamagePlayerCharacter`
  (returns (bCanDamage :type Boolean))
  (bind _playercharacter (`self.PlayerCharacter`))
  ;[1 1 1] Spikes are allowed to damage player if they are overlapping and the player is not in a slow walking state
  (return (and (not (`/Game/MyContent/Blueprints/Characters/Player/BP_PlayerCharacter.IsSlowWalking` _playercharacter)) (`PrimitiveComponent.IsOverlappingActor` (`self.SM_Spikes`) _playercharacter))))

(fn `UserConstructionScript`)