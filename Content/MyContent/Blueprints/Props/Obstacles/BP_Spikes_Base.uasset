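; Base spike obstacle that damages the player on overlap unless they are slow walking.
; Tick checks the overlap against the cached player character and applies spike-typed damage every frame the condition holds.
; The construction script derives lowered and raised Z positions from the mesh and a rise offset.
; MoveSpikesSmoothly lerps the mesh between them by an alpha, with no caller or timeline in this graph.
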(event `self.ReceiveBeginPlay`
  ;[1 1 1] Get reference to player
  (set `self.PlayerCharacter` (cast `/Game/MyContent/Blueprints/Characters/Player/BP_PlayerCharacter` (`GameplayStatics.GetPlayerCharacter` 0) :!pure true)))

(event `self.ReceiveTick`
  (params (DeltaSeconds :type "Float (single-precision)"))
  ;[1 1 1] Damage player if possible
  (if (`self.CanDamagePlayerCharacter`)
    (`GameplayStatics.ApplyDamage` (`self.PlayerCharacter`) (`self.SpikesDamage`) null self "/Game/MyContent/Blueprints/DamageTypes/BP_DamageType_Spikes.BP_DamageType_Spikes_C")))

(fn `CanDamagePlayerCharacter`
  (returns (bCanDamage :type Boolean))
  (bind _playercharacter (`self.PlayerCharacter`))
  ;[1 1 1] Spikes are allowed to damage player if they are overlapping and the player is not in a slow walking state
  (return (and (not (`/Game/MyContent/Blueprints/Characters/Player/BP_PlayerCharacter.IsSlowWalking` _playercharacter)) (`PrimitiveComponent.IsOverlappingActor` (`self.SM_Spikes`) _playercharacter))))

(fn `MoveSpikesSmoothly`
  (params (`Lerp Alpha` :type "Float (double-precision)"))
  (bind _sm_spikes (`self.SM_Spikes`))
  (bind (_relativelocation_x _relativelocation_y) (`KismetMathLibrary.BreakVector` (`SceneComponent.RelativeLocation` _sm_spikes)))
  ;[1 1 1] Lerp between the initial and final Z position using the timeline's alpha and update the spikes' location
  (`SceneComponent.K2_SetRelativeLocation` _sm_spikes (`KismetMathLibrary.MakeVector` _relativelocation_x _relativelocation_y (`KismetMathLibrary.Lerp` (`self.InitialSpikesZPos`) (`self.FinalSpikesZPos`) `Lerp Alpha`)) false false))

(fn `UserConstructionScript`
  (bind (_relativelocation_x _relativelocation_y _relativelocation_z) (`KismetMathLibrary.BreakVector` (`SceneComponent.RelativeLocation` (`self.SM_Spikes`))))
  ;[1 1 1] Set the initial and final Z position of the spikes to move from/to
  (bind _output_get (set `self.InitialSpikesZPos` _relativelocation_z))
  (set `self.FinalSpikesZPos` (+ _output_get (`self.SpikesGoUpByZ`))))