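; BP_Pickup_Base is a base pickup actor, such as for potions, that governs when and where the player can pick it up.
; Its InteractTrigger overlaps toggle CanPickUp as a BP_PlayerCharacter enters or leaves range.
; CalculateInteractLocationAndRotation checks the player's side along world X, then returns a capsule location offset to that side by PlayerPickupOffset and a matching rotation, without moving the player itself.
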(event `self.Interact Trigger.OnComponentBeginOverlap`
  (params (OverlappedComponent :type "PrimitiveComponent Object Reference") (OtherActor :type "Actor Object Reference") (OtherComp :type "PrimitiveComponent Object Reference") (OtherBodyIndex :type Integer) (bFromSweep :type Boolean) (SweepResult :type "HitResult Structure (by ref)"))
  ;[1 1 1] Only allow player to pick up the potion if they are in the range set by the interact trigger
  (if (`GameplayStatics.ObjectIsA` OtherActor "/Game/MyContent/Blueprints/Characters/Player/BP_PlayerCharacter.BP_PlayerCharacter_C")
    (set `self.CanPickUp` true)))

(event `self.Interact Trigger.OnComponentEndOverlap`
  (params (OverlappedComponent :type "PrimitiveComponent Object Reference") (OtherActor :type "Actor Object Reference") (OtherComp :type "PrimitiveComponent Object Reference") (OtherBodyIndex :type Integer))
  ;[1 1 1] Only allow player to pick up the potion if they are in the range set by the interact trigger
  (if (`GameplayStatics.ObjectIsA` OtherActor "/Game/MyContent/Blueprints/Characters/Player/BP_PlayerCharacter.BP_PlayerCharacter_C")
    (set `self.CanPickUp` false)))

(fn `CalculateInteractLocationAndRotation`
  (params (PlayerCharacter :type "PlayerCharacter Object Reference"))
  (returns (InteractLocation :type "Vector Structure") (InteractRotation :type "Rotator Structure"))
  (bind _returnvalue_x (`KismetMathLibrary.BreakVector` (- (`self.K2_GetActorLocation` PlayerCharacter) (`self.K2_GetActorLocation`))))
  (bind _returnvalue (>= _returnvalue_x 0.0))
  (bind _returnvalue_x_2 (`KismetMathLibrary.BreakVector` (- (`self.K2_GetActorLocation` PlayerCharacter) (- (`self.K2_GetActorLocation`) (`KismetMathLibrary.MakeVector` (`KismetMathLibrary.SelectFloat` (* (`self.PlayerPickupOffset`) -1.0) (`self.PlayerPickupOffset`) _returnvalue))))))
  (return (- (`SceneComponent.RelativeLocation` (`Character.CapsuleComponent` PlayerCharacter)) (`KismetMathLibrary.MakeVector` _returnvalue_x_2)) (`KismetMathLibrary.SelectRotator` (struct :`Yaw` 180.0) (struct) _returnvalue)))

(fn `UserConstructionScript`)