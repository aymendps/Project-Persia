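; Sword pickup prop that the player interacts with to obtain their weapon.
; On interact, if pickup is allowed, it hides the button indicator, eases the player capsule to a computed location and rotation, and plays the pickup montage.
; A montage notify hides the prop and spawns the attached sword through PlayerWeaponManager as the hand reaches it.
; On completion, it notifies the player controller, shows the weapon tutorial prompt and destroys itself.
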(event `self.Interact`
  (params (PlayerCharacter :type "PlayerCharacter Object Reference"))
  (bind (_interactlocation _interactrotation) (`self.CalculateInteractLocationAndRotation` PlayerCharacter))
  (bind _asbp_player_character (cast `/Game/MyContent/Blueprints/Characters/Player/BP_PlayerCharacter` PlayerCharacter :!pure true))
  (if (`self.CanPickUp`)
    ;[1 1 1] Hide button indicator since player executed action
    (`SceneComponent.SetVisibility` (`self.Interact Button Indicator`) false false)
    ;[1 1 1] Move player to appropriate location and rotation to pick up the sword
    (`KismetSystemLibrary.MoveComponentTo` (`Character.CapsuleComponent` PlayerCharacter) _interactlocation _interactrotation true true 0.3 true)
    ;[1 1 1] Pick Up Sword
    (`|PlayMontage` (`Character.Mesh` PlayerCharacter) "/Game/MyContent/Animations/Pickups/AM_PickUpSword.AM_PickUpSword"
      (:`OnCompleted`
        (`/Game/MyContent/Blueprints/GameMode/BP_PlayerController.Event FinishedInteract` (`/Game/MyContent/Blueprints/Characters/Player/BP_PlayerCharacter.PlayerController` _asbp_player_character) true)
        (`/Game/MyContent/Blueprints/Widgets/Tutorials/BP_WeaponTutorialManager.DisplayTutorialPrompt` (`self.WeaponTutorialManager`))
        (`self.K2_DestroyActor`))
      (:`OnNotifyBegin`
        ;[1 1 1] When player's hand reaches the sword, hide this pick up and spawn the actual sword that's attached to the player
        (`self.SetActorHiddenInGame` true)
        (`/Game/MyContent/Blueprints/Components/AC_PlayerWeaponManager.SpawnSword` (`/Game/MyContent/Blueprints/Characters/Player/BP_PlayerCharacter.PlayerWeaponManager` _asbp_player_character) true)))))

(fn `UserConstructionScript`)