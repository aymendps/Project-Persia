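; Base potion pickup Blueprint that lets the player pick up and drink a potion, leaving the effect to child Blueprints.
; Interact, gated by CanPickUp, hides the button indicator, eases the player into position and plays the pickup montage.
; Montage notifies attach the potion to the hand socket, then start the drinking animation.
; Children override PotionIsAttached and TriggerPotionEffect, the latter firing after a delay equal to the drink animation's length.
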(event `self.Interact`
  (params (PlayerCharacter :type "PlayerCharacter Object Reference"))
  (bind _asbp_player_character (cast `/Game/MyContent/Blueprints/Characters/Player/BP_PlayerCharacter` PlayerCharacter :!pure true))
  (bind (_interactlocation _interactrotation) (`self.CalculateInteractLocationAndRotation` _asbp_player_character))
  (bind _mesh (`Character.Mesh` _asbp_player_character))
  ;[1 1 1] Interact Implementation - Pick up potioin, drink it, and trigger its effect
  (if (`self.CanPickUp`)
    ;;[1 1 1] Hide button indicator since player executed action
    (`SceneComponent.SetVisibility` (`self.Interact Button Indicator`) false false)
    ;;[1 1 1] Move player to appropriate location and rotation to pick up the potion
    (`KismetSystemLibrary.MoveComponentTo` (`Character.CapsuleComponent` _asbp_player_character) _interactlocation _interactrotation true true 0.3 true)
    (`|PlayMontage` _mesh "/Game/MyContent/Animations/Pickups/AM_PickUp.AM_PickUp"
      (:`OnNotifyBegin`
        ;;[1 1 1] Attach potion to player's hand at the right frame
        (`self.K2_AttachToComponent` _mesh "potion_r_socket" "SnapToTarget" "SnapToTarget" "KeepWorld" false)
        (`self.PotionIsAttached` _asbp_player_character))
      (:`OnNotifyEnd`
        ;;[1 1 1] Drink the potion and trigger its effect afterwards
        (bind _returnvalue (`Character.PlayAnimMontage` _asbp_player_character "/Game/MyContent/Animations/Pickups/AM_Drinking.AM_Drinking" 1.0 "None"))
        (`KismetSystemLibrary.Delay` _returnvalue)
        (`self.TriggerPotionEffect` _asbp_player_character)))))

(event `PotionIsAttached`
  (params (PlayerCharacter :type "/Game/MyContent/Blueprints/Characters/Player/BP_PlayerCharacter Object Reference"))
  ;[1 1 1] These events are to be overriden in child potion blueprints.
  ; PotionIsAttached - Called when potion is attached to player's hand while picking it up.
  ; TriggerPotionEffect - Called when potion should trigger its effect (heal, dmg..).
)

(event `TriggerPotionEffect`
  (params (PlayerCharacter :type "/Game/MyContent/Blueprints/Characters/Player/BP_PlayerCharacter Object Reference"))
  ;[1 1 1] These events are to be overriden in child potion blueprints.
  ; PotionIsAttached - Called when potion is attached to player's hand while picking it up.
  ; TriggerPotionEffect - Called when potion should trigger its effect (heal, dmg..).
)

(fn `UserConstructionScript`)