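; BP_Potion_MaxHP is a potion pickup that permanently raises the player's maximum health.
; When attached, it destroys its surrounding red Niagara particles.
; Triggering it calls GainMaxHealth on the character's Health component, attaches a healing Niagara effect to the capsule, destroys itself and tells the player controller the interaction finished.
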(event `self.PotionIsAttached`
  (params (PlayerCharacter :type "/Game/MyContent/Blueprints/Characters/Player/BP_PlayerCharacter Object Reference"))
  ;[1 1 1] Destroy the red particles surrounding the potion when picked up
  (`ActorComponent.K2_DestroyComponent` (`self.NS Max HP`)))

(event `self.TriggerPotionEffect`
  (params (PlayerCharacter :type "/Game/MyContent/Blueprints/Characters/Player/BP_PlayerCharacter Object Reference"))
  ;[1 1 1] Increase max health and spawn the appropriate particles
  (`HealthComponent.GainMaxHealth` (`/Game/MyContent/Blueprints/Characters/Player/BP_PlayerCharacter.Health` PlayerCharacter) (`self.GainedHealth`))
  (`NiagaraFunctionLibrary.SpawnSystemAttached` "/Game/PickUpSet/Fx/NiagaraSystems/NS_Healing_2.NS_Healing_2" (`Character.CapsuleComponent` PlayerCharacter) "None" (0.0 0.0 20.0) (struct) "KeepRelativeOffset" true)
  (`self.K2_DestroyActor`)
  (`/Game/MyContent/Blueprints/GameMode/BP_PlayerController.Event FinishedInteract` (cast `/Game/MyContent/Blueprints/GameMode/BP_PlayerController` (`GameplayStatics.GetPlayerController` 0) :!pure true) false))

(fn `UserConstructionScript`)