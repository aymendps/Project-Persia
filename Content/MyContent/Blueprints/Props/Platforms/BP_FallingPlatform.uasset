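; BP_FallingPlatform is a platform prop that shakes and then breaks apart after the player steps into its trigger box.
; The first player overlap plays a one-shot timeline at a configurable speed, offsetting the static mesh from a cached initial location.
; When the timeline finishes, the mesh is destroyed and eight separate components start simulating physics.
; The actor can optionally destroy itself after a delay.
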(event `self.Trigger Box.OnComponentBeginOverlap`
  (params (OverlappedComponent :type "PrimitiveComponent Object Reference") (OtherActor :type "Actor Object Reference") (OtherComp :type "PrimitiveComponent Object Reference") (OtherBodyIndex :type Integer) (bFromSweep :type Boolean) (SweepResult :type "HitResult Structure (by ref)"))
  ;[1 1 1] Shake platform for some time and then fall when player enters the trigger box
  ;;[1 1 1] Only proceed if the player did not enter the trigger box yet
  (if (not (`self.IsActivated`))
    (cast `/Game/MyContent/Blueprints/Characters/Player/BP_PlayerCharacter` OtherActor)
    (set `self.IsActivated` true)
    ;;[1 1 1] Shake the platform over time, and then enable physics simulation so that it falls
    (bind (_direction _shake_height) (`Timeline|Shake Timeline`)
      (:`Update`
        (`self.Upate Relative Location` _shake_height))
      (:`Finished`
        (`ActorComponent.K2_DestroyComponent` (`self.StaticMeshComponent`))
        (for _array_element (`self.SimulateWhenDestroyed`)
          (`PrimitiveComponent.SetSimulatePhysics` _array_element true))
        (if (`self.ShouldDestroyActor`)
          (`KismetSystemLibrary.Delay` (`self.DestoryActorAfter`))
          (`self.K2_DestroyActor`))))))

(fn `Upate Relative Location`
  (params (`Shake Height` :type "Vector Structure"))
  (`SceneComponent.K2_SetRelativeLocation` (`self.StaticMeshComponent`) (+ `Shake Height` (`self.InitialLocation`)) false false))

(fn `UserConstructionScript`
  (set `self.InitialLocation` (`self.K2_GetActorLocation`))
  (`TimelineComponent.SetPlayRate` (`self.Shake Timeline`) (`self.ShakeSpeed`))
  (set `self.SimulateWhenDestroyed` (`|MakeArray` (`self.D8`) (`self.D7`) (`self.D6`) (`self.D5`) (`self.D4`) (`self.D3`) (`self.D2`) (`self.D1`))))