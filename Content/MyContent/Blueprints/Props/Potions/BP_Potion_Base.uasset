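; Base potion prop that the player can pick up and drink while inside its interact trigger.
; Interact eases the player's capsule to an X-axis offset and matching rotation on their side of the potion while playing the pick-up montage.
; Montage notifies attach the potion to the hand socket, then start drinking, with the effect firing after that animation's duration.
; Child potions override PotionIsAttached and TriggerPotionEffect to define behavior.
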(event `self.Interact Trigger.OnComponentBeginOverlap`
  (params (OverlappedComponent :type "PrimitiveComponent Object Reference") (OtherActor :type "Actor Object Reference") (OtherComp :type "PrimitiveComponent Object Reference") (OtherBodyIndex :type Integer) (bFromSweep :type Boolean) (SweepResult :type "HitResult Structure (by ref)"))
  ;[1 1 1] Only allow player to pick up the potion if they are in the range set by the interact trigger
  (if (`GameplayStatics.ObjectIsA` OtherActor "/Game/MyContent/Blueprints/Characters/Player/BP_PlayerCharacter.BP_PlayerCharacter_C")
    (set `self.CanPickUp` true)))

(event `self.Interact Trigger.OnComponentEndOverlap`
  (params (OverlappedComponent :type "PrimitiveComponent Object Reference") (OtherActor :type "Actor Object Reference") (OtherComp :type "PrimitiveComponent Object Reference") (OtherBodyIndex :type Integer))
  ;[1 1 1] Only allow player to pick up the potion if they are in the range set by the interact trigger
  (if (`GameplayStatics.ObjectIsA` OtherActor "/Game/MyContent/Blueprints/Characters/Player/BP_PlayerCharacter.BP_PlayerCharacter_C")
    (set `self.CanPickUp` false)))

(event `self.Interact`
  (params (PlayerCharacter :type "PlayerCharacter Object Reference"))
  (bind _asbp_player_character (cast `/Game/MyContent/Blueprints/Characters/Player/BP_PlayerCharacter` PlayerCharacter :!pure true))
  (bind (_interactlocation _interactrotation) (`self.CalculateInteractLocationAndRotation` _asbp_player_character))
  (bind _mesh (`Character.Mesh` _asbp_player_character))
  ;[1 1 1] Interact Implementation - Pick up potioin, drink it, and trigger its effect
  (if (`self.CanPickUp`)
    ;;[1 1 1] Move player to appropriate location and rotation to pick up the potion
    (`KismetSystemLibrary.MoveComponentTo` (`Character.CapsuleComponent` _asbp_player_character) _interactlocation _interactrotation true true 0.3 true)
    (`|PlayMontage` _mesh "/Game/MyContent/Animations/PotionRelated/AM_PickUp.AM_PickUp"
      (:`OnNotifyBegin`
        ;;[1 1 1] Attach potion to player's hand at the right frame
        (`self.K2_AttachToComponent` _mesh "potion_r_socket" "SnapToTarget" "SnapToTarget" "KeepWorld" false)
        (`self.PotionIsAttached` _asbp_player_character))
      (:`OnNotifyEnd`
        ;;[1 1 1] Drink the potion and trigger its effect afterwards
        (bind _returnvalue (`Character.PlayAnimMontage` _asbp_player_character "/Game/MyContent/Animations/PotionRelated/AM_Drinking.AM_Drinking" 1.0 "None"))
        (`KismetSystemLibrary.Delay` _returnvalue)
        (`self.TriggerPotionEffect` _asbp_player_character)))))

(event `PotionIsAttached`
  (params (PlayerCharacter :type "/Game/MyContent/Blueprints/Characters/Player/BP_PlayerCharacter Object Reference"))
  ;[1 1 1] These events are to be overriden in child potion blueprints.
  ; PotionIsAttached - Called when potion is attached to player's hand while picking it up.
  ; TriggerPotionEffect - Called when potion should trigger its effect (heal, dmg..).
)

(event `TriggerPotionEffect`
  (params (PlayerCharacter :type "/Game/MyContent/Blueprints/Characters/Player/BP_PlayerCharacter Object Reference"))
  ;[1 1 1] These events are to be overriden in child potion blueprints.
  ; PotionIsAttached - Called when potion is attached to player's hand while picking it up.
  ; TriggerPotionEffect - Called when potion should trigger its effect (heal, dmg..).
)

(fn `CalculateInteractLocationAndRotation`
  (params (PlayerCharacter :type "/Game/MyContent/Blueprints/Characters/Player/BP_PlayerCharacter Object Reference"))
  (returns (InteractLocation :type "Vector Structure") (InteractRotation :type "Rotator Structure"))
  (bind _returnvalue_x (`KismetMathLibrary.BreakVector` (- (`self.K2_GetActorLocation` PlayerCharacter) (`self.K2_GetActorLocation`))))
  (bind _returnvalue (>= _returnvalue_x 0.0))
  (bind _returnvalue_x_2 (`KismetMathLibrary.BreakVector` (- (`self.K2_GetActorLocation` PlayerCharacter) (- (`self.K2_GetActorLocation`) (`KismetMathLibrary.MakeVector` (`KismetMathLibrary.SelectFloat` (* (`self.PlayerPickupOffset`) -1.0) (`self.PlayerPickupOffset`) _returnvalue))))))
  (return (- (`SceneComponent.RelativeLocation` (`Character.CapsuleComponent` PlayerCharacter)) (`KismetMathLibrary.MakeVector` _returnvalue_x_2)) (`KismetMathLibrary.SelectRotator` (struct :`Yaw` 180.0) (struct) _returnvalue)))

(fn `UserConstructionScript`)