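; BP_EnemyWeapon is a melee weapon prop for enemies that deals sword damage to the player character.
; When its hit collider overlaps the player, it applies damage only while the enemy AI controller's CanAttackDealDamage flag is set.
; It then clears that flag, so one swing cannot hit twice, and resets the AI's hits-taken-in-a-row key to zero.
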(event `self.Hit Collider.OnComponentBeginOverlap`
  (params (OverlappedComponent :type "PrimitiveComponent Object Reference") (OtherActor :type "Actor Object Reference") (OtherComp :type "PrimitiveComponent Object Reference") (OtherBodyIndex :type Integer) (bFromSweep :type Boolean) (SweepResult :type "HitResult Structure (by ref)"))
  (bind _aicontroller (`/Game/MyContent/Blueprints/Characters/Enemy/AI_EnemyCharacter.AIController` (`self.EnemyCharacter`)))
  (if (`/Game/MyContent/Blueprints/Characters/Enemy/AIC_EnemyCharacter.CanAttackDealDamage` (`/Game/MyContent/Blueprints/Characters/Enemy/AI_EnemyCharacter.AIController` (`self.EnemyCharacter`)))
    ;[1 1 1] Deal damage and then switch can attack deal damage back to false to avoid dealing extra damage when the weapon passes more than once through the player in the same attack. Reset hits taken in row to 0 since the AI is the one who dealt damage just now
    (bind _asbp_player_character (cast `/Game/MyContent/Blueprints/Characters/Player/BP_PlayerCharacter` OtherActor))
    (`GameplayStatics.ApplyDamage` _asbp_player_character (`self.WeaponDamage`) (`/Game/MyContent/Blueprints/Characters/Enemy/AI_EnemyCharacter.AIController` (`self.EnemyCharacter`)) self "/Game/MyContent/Blueprints/DamageTypes/BP_DamageType_Sword.BP_DamageType_Sword_C")
    (set `/Game/MyContent/Blueprints/Characters/Enemy/AIC_EnemyCharacter.CanAttackDealDamage` false _aicontroller)
    (`/Game/MyContent/Blueprints/Characters/Enemy/AIC_EnemyCharacter.UpdateHitsTakenInRowKey` _aicontroller 0)))

(fn `UserConstructionScript`
  (`parent.UserConstructionScript`))