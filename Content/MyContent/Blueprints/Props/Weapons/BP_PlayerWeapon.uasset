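; BP_PlayerWeapon is the player's melee weapon that damages enemy AI through its hit collider.
; On overlap during an active attack window, it applies sword-type damage to an AI_EnemyCharacter, then clears the player's CanAttackDealDamage flag so each attack hits only once.
; If the enemy's AI controller is parrying, it skips damage and triggers the player's parried reaction instead.
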(event `self.Hit Collider.OnComponentBeginOverlap`
  (params (OverlappedComponent :type "PrimitiveComponent Object Reference") (OtherActor :type "Actor Object Reference") (OtherComp :type "PrimitiveComponent Object Reference") (OtherBodyIndex :type Integer) (bFromSweep :type Boolean) (SweepResult :type "HitResult Structure (by ref)"))
  (if (`/Game/MyContent/Blueprints/Characters/Player/BP_PlayerCharacter.CanAttackDealDamage` (`self.PlayerCharacter`))
    (bind _asai_enemy_character (cast `/Game/MyContent/Blueprints/Characters/Enemy/AI_EnemyCharacter` OtherActor))
    (if (not (`/Game/MyContent/Blueprints/Characters/Enemy/AIC_EnemyCharacter.IsParrying` (`/Game/MyContent/Blueprints/Characters/Enemy/AI_EnemyCharacter.AIController` _asai_enemy_character)))
      ;[1 1 1] Deal damage and then switch can attack deal damage back to false to avoid dealing extra damage when the weapon passes more than once through the enemy AI in the same attack
      (`GameplayStatics.ApplyDamage` _asai_enemy_character (`self.WeaponDamage`) (`/Game/MyContent/Blueprints/Characters/Player/BP_PlayerCharacter.PlayerController` (`self.PlayerCharacter`)) self "/Game/MyContent/Blueprints/DamageTypes/BP_DamageType_Sword.BP_DamageType_Sword_C")
      (set `/Game/MyContent/Blueprints/Characters/Player/BP_PlayerCharacter.CanAttackDealDamage` false (`self.PlayerCharacter`))
      (else
        ;[1 1 1] Since AI did a successful parry, don't apply damage. Instead make the player react to the parry
        (`/Game/MyContent/Blueprints/Characters/Player/BP_PlayerCharacter.PlayerWasParried` (`self.PlayerCharacter`))))))

(fn `UserConstructionScript`
  (`parent.UserConstructionScript`))